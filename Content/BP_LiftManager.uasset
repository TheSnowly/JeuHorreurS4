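; Lift manager that spawns a lift corridor on BeginPlay and immediately starts a timed lift ride sequence.
; Starting sets the gear actors (Rouages) rotating and arms a ten-second timer that stops them and halves the shake intensity.
; Tick restarts the player camera shake every frame while LiftMoving is set, which is never cleared here.
; A separate event plays an end-of-lift shake.
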(event `self.ReceiveBeginPlay`
  (bind _returnvalue (`|SpawnActorFromClass` "/Game/BP_LiftCorridor.BP_LiftCorridor_C" (`KismetMathLibrary.Conv_VectorToTransform` (`KismetMathLibrary.Vector_Zero`)) "Undefined" "MultiplyWithRoot" null null))
  (set `self.LiftCorridor` _returnvalue)
  (`self.StartLift`))

(event `StartLift`
  (set `self.ScaleLiftCameraShake` 0.5)
  (set `self.LiftMoving` true)
  (for _array_element (`self.Rouages`)
    (set `/Game/BP_Rouage.Rotate` true _array_element)
    (`self.Timer`)))

(event `ShakeEndLift`
  (`PlayerController.ClientStartCameraShake` :`self` (`GameplayStatics.GetPlayerController` 0) :`Shake` "/Game/CameraShakeLiftEnd.CameraShakeLiftEnd_C"))

(event `Timer`
  (`KismetSystemLibrary.K2_SetTimerDelegate` (delegate `EndLift`) 10.0))

(event `EndLift`
  (set `self.ScaleLiftCameraShake` 0.25)
  (for _array_element (`self.Rouages`)
    (set `/Game/BP_Rouage.Rotate` false _array_element)
    (`/Game/BP_Rouage.EndLiftRotate` _array_element)))

(event `self.ReceiveTick`
  (params (DeltaSeconds :type "Float (single-precision)"))
  (if (`self.LiftMoving`)
    (`PlayerController.ClientStartCameraShake` :`self` (`GameplayStatics.GetPlayerController` 0) :`Shake` "/Game/CameraShakeLift.CameraShakeLift_C" :`Scale` (`self.ScaleLiftCameraShake`))))

(fn `UserConstructionScript`)