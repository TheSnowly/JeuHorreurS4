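; Interactable roulette that, once per play, takes control of BP_FP and stages a scripted first-person spin sequence.
; BeginPlay sphere-traces downward for two standing spots in front of the mesh.
; Chained timelines move the player in, swing the spring arm up and down to mimic the spinning motion, then step back and restore control.
; An event track on the downswing starts the spin, which Tick decelerates with a growing lerp alpha.
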(event `self.ReceiveBeginPlay`
  (bind _staticmeshcomponent1 (`self.StaticMeshComponent1`))
  (bind _returnvalue (`SceneComponent.K2_GetComponentLocation` _staticmeshcomponent1))
  (bind _returnvalue_2 (`SceneComponent.GetForwardVector` _staticmeshcomponent1))
  (bind _returnvalue_3 (+ _returnvalue (* _returnvalue_2 150.0)))
  (bind _returnvalue_4 (+ _returnvalue (* _returnvalue_2 80.0)))
  (bind _outhit (`KismetSystemLibrary.SphereTraceSingle` _returnvalue_4 (- _returnvalue_4 (0.0 0.0 400.0)) 5.0 "TraceTypeQuery1"))
  (set `self.PlayerDesiredLocation` (`.Location` (`GameplayStatics.BreakHitResult` _outhit)))
  (bind _outhit_2 (`KismetSystemLibrary.SphereTraceSingle` _returnvalue_3 (- _returnvalue_3 (0.0 0.0 400.0)) 5.0 "TraceTypeQuery1"))
  (set `self.PlayerDesiredRotationTwo` (`.Location` (`GameplayStatics.BreakHitResult` _outhit_2))))

(event `/Game/FirstPerson/Blueprints/BPI_Interact.Interact`
  (bind (_playerdesiredrotationtwo_x _playerdesiredrotationtwo_y) (`KismetMathLibrary.BreakVector` (`self.PlayerDesiredRotationTwo`)))
  (bind (_playerdesiredlocation_x _playerdesiredlocation_y) (`KismetMathLibrary.BreakVector` (`self.PlayerDesiredLocation`)))
  (bind _bp_firstperson (`self.BP_FirstPerson`))
  (bind (_rouetteactiondesiredrotation_roll _rouetteactiondesiredrotation_pitch _rouetteactiondesiredrotation_yaw) (`KismetMathLibrary.BreakRotator` (`self.RouetteActionDesiredRotation`)))
  (bind _capsulecomponent (`Character.CapsuleComponent` (`self.BP_FirstPerson`)))
  (bind _springarm (`/Game/FirstPerson/Blueprints/BP_FP.SpringArm` (`self.BP_FirstPerson`)))
  (bind _springarm_2 (`/Game/FirstPerson/Blueprints/BP_FP.SpringArm` (`self.BP_FirstPerson`)))
  (bind _springarm_3 (`/Game/FirstPerson/Blueprints/BP_FP.SpringArm` (`self.BP_FirstPerson`)))
  (bind _capsulecomponent_2 (`Character.CapsuleComponent` (`self.BP_FirstPerson`)))
  (bind (_returnvalue_x _returnvalue_y _returnvalue_z) (`KismetMathLibrary.BreakVector` (`SceneComponent.K2_GetComponentLocation` _capsulecomponent)))
  (bind (_returnvalue_x_2 _returnvalue_y_2 _returnvalue_z_2) (`KismetMathLibrary.BreakVector` (`SceneComponent.K2_GetComponentLocation` _capsulecomponent_2)))
  (bind (_relativerotation_roll _relativerotation_pitch _relativerotation_yaw) (`KismetMathLibrary.BreakRotator` (`SceneComponent.RelativeRotation` _springarm_3)))
  (`/Engine/EditorBlueprintResources/StandardMacros.DoOnce` false
    (:`Completed`
      (bind _returnvalue (`GameplayStatics.GetActorOfClass` "/Game/FirstPerson/Blueprints/BP_FP.BP_FP_C"))
      (bind _output_get (set `self.BP_FirstPerson` _returnvalue))
      (set `/Game/FirstPerson/Blueprints/BP_FP.IsDoingInteractAction` true _output_get)
      (set `SpringArmComponent.bUsePawnControlRotation` false (`/Game/FirstPerson/Blueprints/BP_FP.SpringArm` _output_get))
      (`CharacterMovementComponent.DisableMovement` (`Character.CharacterMovement` _output_get))
      (`TimelineComponent.SetPlayRate` (`self.MovePlayer`) 0.4)
      (bind (_direction _move) (`Timeline|MovePlayer` :!via `PlayFromStart`)
        (:`Update`
          (`SceneComponent.K2_SetWorldLocation` _capsulecomponent (`KismetMathLibrary.MakeVector` (`KismetMathLibrary.Lerp` _returnvalue_x _playerdesiredlocation_x _move) (`KismetMathLibrary.Lerp` _returnvalue_y _playerdesiredlocation_y _move) _returnvalue_z) false false)
          (`SceneComponent.K2_SetWorldRotation` _springarm (`KismetMathLibrary.RLerp` (`SceneComponent.K2_GetComponentRotation` _springarm) (`KismetMathLibrary.FindLookAtRotation` (`SceneComponent.K2_GetComponentLocation` _springarm) (`SceneComponent.K2_GetComponentLocation` (`self.r`))) _move true) false false))
        (:`Finished`
          (set `self.SpringArmBaseRotation` (`SceneComponent.K2_GetComponentRotation` _springarm_3))
          (set `self.RouletteActionBaseRotation` (`KismetMathLibrary.MakeRotator` _relativerotation_roll _relativerotation_pitch _relativerotation_yaw))
          (set `self.RouetteActionDesiredRotation` (`KismetMathLibrary.MakeRotator` _relativerotation_roll (+ _relativerotation_pitch 30.0) (+ _relativerotation_yaw 60.0)))
          (`TimelineComponent.SetPlayRate` (`self.rotateHeadUp`) 0.7)
          (bind (_direction_2 _newtrack_0) (`Timeline|rotateHeadUp`)
            (:`Update`
              (`SceneComponent.K2_SetRelativeRotation` (`/Game/FirstPerson/Blueprints/BP_FP.SpringArm` (`self.BP_FirstPerson`)) (`KismetMathLibrary.RLerp` (`self.RouletteActionBaseRotation`) (`self.RouetteActionDesiredRotation`) _newtrack_0) false false))
            (:`Finished`
              (set `self.RouletteActionBaseRotation` (`KismetMathLibrary.MakeRotator` _rouetteactiondesiredrotation_roll (- _rouetteactiondesiredrotation_pitch 100.0) _rouetteactiondesiredrotation_yaw))
              (`TimelineComponent.SetPlayRate` (`self.RotateHeadDown`) 5.0)
              (bind (_direction_3 _newtrack_0_2) (`Timeline|RotateHeadDown` :!via `PlayFromStart`)
                (:`Update`
                  (`SceneComponent.K2_SetRelativeRotation` (`/Game/FirstPerson/Blueprints/BP_FP.SpringArm` (`self.BP_FirstPerson`)) (`KismetMathLibrary.RLerp` (`self.RouetteActionDesiredRotation`) (`self.RouletteActionBaseRotation`) _newtrack_0_2) false false))
                (:`Finished`
                  (`KismetSystemLibrary.Delay` 0.5)
                  (`TimelineComponent.SetPlayRate` (`self.ReturnToPosition`) 0.1)
                  (bind (_direction_4 _move_2) (`Timeline|ReturnToPosition` :!via `PlayFromStart`)
                    (:`Update`
                      (`SceneComponent.K2_SetWorldLocation` _capsulecomponent_2 (`KismetMathLibrary.MakeVector` (`KismetMathLibrary.Lerp` _returnvalue_x_2 _playerdesiredrotationtwo_x _move_2) (`KismetMathLibrary.Lerp` _returnvalue_y_2 _playerdesiredrotationtwo_y _move_2) _returnvalue_z_2) false false)
                      (`SceneComponent.K2_SetWorldRotation` _springarm_2 (`KismetMathLibrary.RLerp` (`SceneComponent.K2_GetComponentRotation` _springarm_2) (`KismetMathLibrary.FindLookAtRotation` (`SceneComponent.K2_GetComponentLocation` _springarm_2) (`SceneComponent.K2_GetComponentLocation` (`self.r`))) _move_2 true) false false))
                    (:`Finished`
                      (set `/Game/FirstPerson/Blueprints/BP_FP.IsDoingInteractAction` false _bp_firstperson)
                      (set `SpringArmComponent.bUsePawnControlRotation` true (`/Game/FirstPerson/Blueprints/BP_FP.SpringArm` _bp_firstperson))
                      (`CharacterMovementComponent.SetMovementMode` (`Character.CharacterMovement` _bp_firstperson) "MOVE_Walking" 0))))
                (:`TurnRoulette`
                  (set `self.RotationSpeed` -40.0)
                  (set `self.RouletteTurning` true))))))))))

(event `self.ReceiveTick`
  (params (DeltaSeconds :type "Float (single-precision)"))
  (if (`self.RouletteTurning`)
    (`SceneComponent.K2_AddLocalRotation` (`self.r`) (`KismetMathLibrary.MakeRotator` 0.0 0.0 (`self.RotationSpeed`)) false false)
    (set `self.RotationSpeed` (`KismetMathLibrary.Lerp` (`self.RotationSpeed`) 0.0 (`self.AlphaRotationSpeed`)))
    (set `self.AlphaRotationSpeed` (+ (`self.AlphaRotationSpeed`) 2e-05))
    (if (>= (`self.RotationSpeed`) 0.0)
      (set `self.RouletteTurning` false))))

(fn `UserConstructionScript`)