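; BP_Test is a one-time interactable lever that plays a scripted first-person pull sequence.
; BeginPlay sphere-traces downward in front of its mesh to store the player's standing spot.
; Interact locks BP_FP's movement and spring arm, then the MovePlayer timeline eases the capsule there and turns the view toward the mesh.
; The ActivateLever timeline then tilts the view pitch, snaps Wa to its pulled pose on an event track, and restores control.
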(event `self.ReceiveBeginPlay`
  (bind _staticmeshcomponent1 (`self.StaticMeshComponent1`))
  (bind _returnvalue (+ (`SceneComponent.K2_GetComponentLocation` _staticmeshcomponent1) (* (`SceneComponent.GetForwardVector` _staticmeshcomponent1) 100.0)))
  (bind _outhit (`KismetSystemLibrary.SphereTraceSingle` _returnvalue (- _returnvalue (0.0 0.0 400.0)) 5.0 "TraceTypeQuery1"))
  (set `self.PlayerDesiredLocation` (`.Location` (`GameplayStatics.BreakHitResult` _outhit))))

(event `/Game/FirstPerson/Blueprints/BPI_Interact.Interact`
  (bind _wa (`self.wa`))
  (bind _bp_firstperson (`self.BP_FirstPerson`))
  (bind (_playerdesiredlocation_x _playerdesiredlocation_y) (`KismetMathLibrary.BreakVector` (`self.PlayerDesiredLocation`)))
  (bind (_returnvalue_x _returnvalue_y _returnvalue_z) (`KismetMathLibrary.BreakVector` (`SceneComponent.K2_GetComponentLocation` _wa)))
  (bind _springarm (`/Game/FirstPerson/Blueprints/BP_FP.SpringArm` (`self.BP_FirstPerson`)))
  (bind _springarm_2 (`/Game/FirstPerson/Blueprints/BP_FP.SpringArm` (`self.BP_FirstPerson`)))
  (bind _capsulecomponent (`Character.CapsuleComponent` (`self.BP_FirstPerson`)))
  (bind (_returnvalue_x_2 _returnvalue_y_2 _returnvalue_z_2) (`KismetMathLibrary.BreakVector` (`SceneComponent.K2_GetComponentLocation` _capsulecomponent)))
  (bind (_relativerotation_roll _relativerotation_pitch _relativerotation_yaw) (`KismetMathLibrary.BreakRotator` (`SceneComponent.RelativeRotation` _springarm)))
  (`/Engine/EditorBlueprintResources/StandardMacros.DoOnce` false
    (:`Completed`
      (bind _returnvalue (`GameplayStatics.GetActorOfClass` "/Game/FirstPerson/Blueprints/BP_FP.BP_FP_C"))
      (bind _output_get (set `self.BP_FirstPerson` _returnvalue))
      (set `/Game/FirstPerson/Blueprints/BP_FP.IsDoingInteractAction` true _output_get)
      (set `SpringArmComponent.bUsePawnControlRotation` false (`/Game/FirstPerson/Blueprints/BP_FP.SpringArm` _output_get))
      (`CharacterMovementComponent.DisableMovement` (`Character.CharacterMovement` _output_get))
      (`TimelineComponent.SetPlayRate` (`self.MovePlayer`) 0.4)
      (bind (_direction _move) (`Timeline|MovePlayer` :!via `PlayFromStart`)
        (:`Update`
          (`SceneComponent.K2_SetWorldLocation` _capsulecomponent (`KismetMathLibrary.MakeVector` (`KismetMathLibrary.Lerp` _returnvalue_x_2 _playerdesiredlocation_x _move) (`KismetMathLibrary.Lerp` _returnvalue_y_2 _playerdesiredlocation_y _move) _returnvalue_z_2) false false)
          (`SceneComponent.K2_SetWorldRotation` _springarm_2 (`KismetMathLibrary.RLerp` (`SceneComponent.K2_GetComponentRotation` _springarm_2) (`KismetMathLibrary.FindLookAtRotation` (`SceneComponent.K2_GetComponentLocation` _springarm_2) (`SceneComponent.K2_GetComponentLocation` (`self.StaticMeshComponent1`))) _move true) false false))
        (:`Finished`
          (set `self.DesiredRotationPitch` (+ _relativerotation_pitch 60.0))
          (set `self.CurrentRotationPitch` _relativerotation_pitch)
          (`TimelineComponent.SetPlayRate` (`self.ActivateLever`) 0.7)
          (bind (_direction_2 _move_2) (`Timeline|ActivateLever` :!via `PlayFromStart`)
            (:`Update`
              (`SceneComponent.K2_SetRelativeRotation` _springarm (`KismetMathLibrary.MakeRotator` _relativerotation_roll (`KismetMathLibrary.Lerp` (`self.CurrentRotationPitch`) (`self.DesiredRotationPitch`) _move_2) _relativerotation_yaw) false false))
            (:`Finished`
              (set `/Game/FirstPerson/Blueprints/BP_FP.IsDoingInteractAction` false _bp_firstperson)
              (set `SpringArmComponent.bUsePawnControlRotation` true (`/Game/FirstPerson/Blueprints/BP_FP.SpringArm` _bp_firstperson))
              (`CharacterMovementComponent.SetMovementMode` (`Character.CharacterMovement` _bp_firstperson) "MOVE_Walking" 0))
            (:`PullLever`
              (`SceneComponent.K2_SetRelativeRotation` _wa (struct :`Yaw` -90.0 :`Roll` 40.0) false false)
              (`SceneComponent.K2_SetWorldLocation` _wa (`KismetMathLibrary.MakeVector` _returnvalue_x _returnvalue_y (- _returnvalue_z 20.0)) false false))))))))

(fn `UserConstructionScript`)