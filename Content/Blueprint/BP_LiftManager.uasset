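; BP_LiftManager runs a timed lift ride that begins at BeginPlay, driving a referenced BPLift and the first player's camera shake.
; Chained timers stop the lift and trigger its end rotation, then open its doors.
; Tick restarts the travel shake every frame, weakened after arrival but never stopped, as LiftMoving is never cleared.
; A separate ShakeEndLift event plays an end shake but is not called here.
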(event `self.ReceiveBeginPlay`
  (`self.StartLift`))

(event `StartLift`
  (set `self.ScaleLiftCameraShake` 0.5)
  (set `self.LiftMoving` true)
  (`self.Timer`)
  (set `/Game/Blueprint/BP_Lift.Moving` true (`self.BP_Lift`)))

(event `ShakeEndLift`
  (`PlayerController.ClientStartCameraShake` :`self` (`GameplayStatics.GetPlayerController` 0) :`Shake` "/Game/Blueprint/CameraShakeLiftEnd.CameraShakeLiftEnd_C"))

(event `Timer`
  (`KismetSystemLibrary.K2_SetTimerDelegate` (delegate `EndLift`) 5.0))

(event `EndLift`
  (bind _bp_lift (`self.BP_Lift`))
  (set `self.ScaleLiftCameraShake` 0.25)
  (set `/Game/Blueprint/BP_Lift.Moving` false _bp_lift)
  (`/Game/Blueprint/BP_Lift.EndLiftRotate` _bp_lift)
  (`KismetSystemLibrary.K2_SetTimerDelegate` (delegate `OpenDoor`) 5.0))

(event `OpenDoor`
  (`/Game/Blueprint/BP_Lift.OpenDoors` (`self.BP_Lift`)))

(event `self.ReceiveTick`
  (params (DeltaSeconds :type "Float (single-precision)"))
  (if (`self.LiftMoving`)
    (`PlayerController.ClientStartCameraShake` :`self` (`GameplayStatics.GetPlayerController` 0) :`Shake` "/Game/Blueprint/CameraShakeLift.CameraShakeLift_C" :`Scale` (`self.ScaleLiftCameraShake`))))

(fn `UserConstructionScript`)