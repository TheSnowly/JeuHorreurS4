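; BP_Lift is a lift actor that animates four gear meshes and two sliding doors.
; While Moving is set, Tick spins the gears by local yaw.
; EndLiftRotate plays a slowed timeline that eases all gears' pitch back 20 degrees from the value sampled on one gear, with event tracks telling LiftManager to shake and clear LiftMoving.
; OpenDoors runs a second timeline sliding the doors apart along Y.
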(event `self.ReceiveTick`
  (params (DeltaSeconds :type "Float (single-precision)"))
  (bind _rouagerotationspeed (`self.RouageRotationSpeed`))
  (if (`self.Moving`)
    (`SceneComponent.K2_AddLocalRotation` (`self.Engrenage_lebon2_StaticMeshComponent0`) (`KismetMathLibrary.MakeRotator` 0.0 0.0 _rouagerotationspeed) false false)
    (`SceneComponent.K2_AddLocalRotation` (`self.Engrenage_lebon3_StaticMeshComponent0`) (`KismetMathLibrary.MakeRotator` 0.0 0.0 _rouagerotationspeed) false false)
    (`SceneComponent.K2_AddLocalRotation` (`self.Engrenage_lebon4_StaticMeshComponent0`) (`KismetMathLibrary.MakeRotator` 0.0 0.0 _rouagerotationspeed) false false)
    (`SceneComponent.K2_AddLocalRotation` (`self.Engrenage_lebon_StaticMeshComponent0`) (`KismetMathLibrary.MakeRotator` 0.0 0.0 _rouagerotationspeed) false false)))

(event `EndLiftRotate`
  (bind _engrenage_lebon2_staticmeshcomponent0 (`self.Engrenage_lebon2_StaticMeshComponent0`))
  (bind _engrenage_lebon3_staticmeshcomponent0 (`self.Engrenage_lebon3_StaticMeshComponent0`))
  (bind _engrenage_lebon4_staticmeshcomponent0 (`self.Engrenage_lebon4_StaticMeshComponent0`))
  (bind _engrenage_lebon_staticmeshcomponent0 (`self.Engrenage_lebon_StaticMeshComponent0`))
  (bind _liftmanager (`self.LiftManager`))
  (bind (_relativerotation_roll _relativerotation_pitch _relativerotation_yaw) (`KismetMathLibrary.BreakRotator` (`SceneComponent.RelativeRotation` _engrenage_lebon2_staticmeshcomponent0)))
  (bind (_relativerotation_roll_2 _relativerotation_pitch_2 _relativerotation_yaw_2) (`KismetMathLibrary.BreakRotator` (`SceneComponent.RelativeRotation` _engrenage_lebon_staticmeshcomponent0)))
  (bind (_relativerotation_roll_3 _relativerotation_pitch_3 _relativerotation_yaw_3) (`KismetMathLibrary.BreakRotator` (`SceneComponent.RelativeRotation` _engrenage_lebon3_staticmeshcomponent0)))
  (bind (_relativerotation_roll_4 _relativerotation_pitch_4 _relativerotation_yaw_4) (`KismetMathLibrary.BreakRotator` (`SceneComponent.RelativeRotation` _engrenage_lebon4_staticmeshcomponent0)))
  (bind (_relativerotation_roll_5 _relativerotation_pitch_5) (`KismetMathLibrary.BreakRotator` (`SceneComponent.RelativeRotation` (`self.Engrenage_lebon2_StaticMeshComponent0`))))
  (set `self.LastRotation` _relativerotation_pitch_5)
  (`TimelineComponent.SetPlayRate` (`self.Timeline`) 0.3)
  (bind (_direction _rotation) (`Timeline|Timeline` :!via `PlayFromStart`)
    (:`Update`
      (bind _returnvalue (`KismetMathLibrary.Lerp` (`self.LastRotation`) (+ (`self.LastRotation`) -20.0) _rotation))
      (`SceneComponent.K2_SetRelativeRotation` _engrenage_lebon2_staticmeshcomponent0 (`KismetMathLibrary.MakeRotator` _relativerotation_roll _returnvalue _relativerotation_yaw) false false)
      (`SceneComponent.K2_SetRelativeRotation` _engrenage_lebon3_staticmeshcomponent0 (`KismetMathLibrary.MakeRotator` _relativerotation_roll_3 _returnvalue _relativerotation_yaw_3) false false)
      (`SceneComponent.K2_SetRelativeRotation` _engrenage_lebon4_staticmeshcomponent0 (`KismetMathLibrary.MakeRotator` _relativerotation_roll_4 _returnvalue _relativerotation_yaw_4) false false)
      (`SceneComponent.K2_SetRelativeRotation` _engrenage_lebon_staticmeshcomponent0 (`KismetMathLibrary.MakeRotator` _relativerotation_roll_2 _returnvalue _relativerotation_yaw_2) false false))
    (:`StopRotation`
      (set `/Game/Blueprint/BP_LiftManager.LiftMoving` false _liftmanager))
    (:`GoDown`
      (`/Game/Blueprint/BP_LiftManager.ShakeEndLift` _liftmanager))))

(event `OpenDoors`
  (bind _porte_gauche_staticmeshcomponent0 (`self.porte_gauche_StaticMeshComponent0`))
  (bind _porte_droite_staticmeshcomponent0 (`self.porte_droite_StaticMeshComponent0`))
  (bind (_relativelocation_x _relativelocation_y _relativelocation_z) (`KismetMathLibrary.BreakVector` (`SceneComponent.RelativeLocation` _porte_droite_staticmeshcomponent0)))
  (bind (_relativelocation_x_2 _relativelocation_y_2 _relativelocation_z_2) (`KismetMathLibrary.BreakVector` (`SceneComponent.RelativeLocation` _porte_gauche_staticmeshcomponent0)))
  (`TimelineComponent.SetPlayRate` (`self.OpenDoor`) 1.5)
  (bind (_direction _newtrack_0) (`Timeline|OpenDoor` :!via `PlayFromStart`)
    (:`Update`
      (bind _returnvalue (* _newtrack_0 200.0))
      (`SceneComponent.K2_SetRelativeLocation` _porte_droite_staticmeshcomponent0 (`KismetMathLibrary.MakeVector` _relativelocation_x (* _returnvalue -1.0) _relativelocation_z) false false)
      (`SceneComponent.K2_SetRelativeLocation` _porte_gauche_staticmeshcomponent0 (`KismetMathLibrary.MakeVector` _relativelocation_x_2 _returnvalue _relativelocation_z_2) false false))))

(fn `UserConstructionScript`)