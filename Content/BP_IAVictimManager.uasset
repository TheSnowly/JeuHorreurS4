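; BP_IAVictimManager is a manager actor that spawns and tracks AI victims.
; On BeginPlay it loops up to NbToSpawn, spawning BP_IA_Victim actors in a row along X from the SpawnZone component and storing them in VictimsArray.
; It then runs Move, which triggers Called on only the first victim in the array.
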(event `self.ReceiveBeginPlay`
  (bind (_returnvalue_x _returnvalue_y _returnvalue_z) (`KismetMathLibrary.BreakVector` (`SceneComponent.K2_GetComponentLocation` (`self.SpawnZone`))))
  (for _index (range (+ (`self.NbToSpawn`) 1))
    (bind _returnvalue (`|SpawnActorFromClass` "/Game/ia/IA_Victim/BP_IA_Victim.BP_IA_Victim_C" (`KismetMathLibrary.MakeTransform` (`KismetMathLibrary.MakeVector` (+ _returnvalue_x (* _index 60.0)) _returnvalue_y _returnvalue_z)) "Undefined" "MultiplyWithRoot" null null))
    (`KismetArrayLibrary.Array_Add` (`self.VictimsArray`) _returnvalue))
  (`self.Move`))

(event `Move`
  (`/Game/ia/IA_Victim/BP_IA_Victim.Called` (`|GetArrayItem` (`self.VictimsArray`))))

(fn `UserConstructionScript`)