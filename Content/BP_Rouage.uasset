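; BP_Rouage is a gear actor for the lift that spins its EngrenageLebon component by a fixed yaw step each Tick while Rotate is true.
; EndLiftRotate plays a slowed timeline that lerps a final 20-degree turn from the current yaw.
; Timeline event tracks call back to the BP_LiftManager found at BeginPlay, clearing LiftMoving and triggering the end-of-lift shake.
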(event `self.ReceiveBeginPlay`
  (bind _returnvalue (`GameplayStatics.GetActorOfClass` "/Game/BP_LiftManager.BP_LiftManager_C"))
  (set `self.LiftManager` _returnvalue))

(event `EndLiftRotate`
  (bind _liftmanager (`self.LiftManager`))
  (bind (_relativerotation_roll _relativerotation_pitch) (`KismetMathLibrary.BreakRotator` (`SceneComponent.RelativeRotation` (`self.Engrenage_lebon`))))
  (bind (_relativerotation_roll_2 _relativerotation_pitch_2 _relativerotation_yaw) (`KismetMathLibrary.BreakRotator` (`SceneComponent.RelativeRotation` (`self.Engrenage_lebon`))))
  (set `self.LastRotation` _relativerotation_yaw)
  (`TimelineComponent.SetPlayRate` (`self.Timeline`) 0.3)
  (bind (_direction _rotation) (`Timeline|Timeline` :!via `PlayFromStart`)
    (:`Update`
      (`SceneComponent.K2_SetRelativeRotation` (`self.Engrenage_lebon`) (`KismetMathLibrary.MakeRotator` _relativerotation_roll _relativerotation_pitch (`KismetMathLibrary.Lerp` (`self.LastRotation`) (+ (`self.LastRotation`) 20.0) _rotation)) false false))
    (:`StopRotation`
      (set `/Game/BP_LiftManager.LiftMoving` false _liftmanager))
    (:`GoDown`
      (`/Game/BP_LiftManager.ShakeEndLift` _liftmanager))))

(event `self.ReceiveTick`
  (params (DeltaSeconds :type "Float (single-precision)"))
  (if (`self.Rotate`)
    (`SceneComponent.K2_AddLocalRotation` (`self.Engrenage_lebon`) (`KismetMathLibrary.MakeRotator` 0.0 0.0 0.3) false false)))

(fn `UserConstructionScript`)