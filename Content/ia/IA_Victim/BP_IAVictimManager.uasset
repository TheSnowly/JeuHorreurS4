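; Manager actor that runs a queue of AI victims, each of which is either killed or saved in turn.
; On BeginPlay it spawns a line of BP_IA_Victim along Y from SpawnZone and calls the front one.
; Kill ragdolls and destroys the front victim after short delays, while Save sends it away with a growing offset.
; Both then remove it from the array and call the next until the array is empty.
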(event `self.ReceiveBeginPlay`
  (bind (_returnvalue_x _returnvalue_y _returnvalue_z) (`KismetMathLibrary.BreakVector` (`SceneComponent.K2_GetComponentLocation` (`self.SpawnZone`))))
  (set `self.OffsetBase` (* (`self.NbToSpawn`) 60))
  (for _index (range (+ (`self.NbToSpawn`) 1))
    (bind _returnvalue (`|SpawnActorFromClass` "/Game/ia/IA_Victim/BP_IA_Victim.BP_IA_Victim_C" (`KismetMathLibrary.MakeTransform` (`KismetMathLibrary.MakeVector` _returnvalue_x (+ _returnvalue_y (* _index 60.0)) _returnvalue_z)) "Undefined" "MultiplyWithRoot" null null))
    (`KismetArrayLibrary.Array_Add` (`self.VictimsArray`) _returnvalue))
  (`self.Move`))

(event `Move`
  (`/Game/ia/IA_Victim/BP_IA_Victim.Called` (`|GetArrayItem` (`self.VictimsArray`))))

(event `Kill`
  (bind _output (`|GetArrayItem` (`self.VictimsArray`)))
  (`KismetSystemLibrary.Delay` 0.4)
  (`PrimitiveComponent.SetSimulatePhysics` (`Character.Mesh` _output) true)
  (`KismetSystemLibrary.Delay` 0.8)
  (`self.K2_DestroyActor` _output)
  (`self.ModifyArray`))

(event `Save`
  (bind _output (`|GetArrayItem` (`self.VictimsArray`)))
  (`KismetSystemLibrary.Delay` 0.4)
  (set `/Game/ia/IA_Victim/BP_IA_Victim.Offset` (`self.OffsetBase`) _output)
  (set `self.OffsetBase` (+ (`self.OffsetBase`) 60))
  (`/Game/ia/IA_Victim/BP_IA_Victim.GoAway` _output)
  (`self.ModifyArray`))

(event `ModifyArray`
  (bind _victimsarray (`self.VictimsArray`))
  (`KismetArrayLibrary.Array_Remove` _victimsarray)
  (if (!= (`KismetArrayLibrary.Array_Length` _victimsarray) 0)
    (`self.Move`)))

(fn `UserConstructionScript`)